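; Checkpoint actor that saves the player's position and rotation, or clears the saved checkpoint, depending on its Load flag.
; Any Box overlap with Load true records the player character's transform into the "check" save slot, creating it if needed, then destroys the actor after a short delay.
; With Load false, the overlap instead sets the existing save's Load flag to false and leaves the actor in place.
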(event `self.Box.OnComponentBeginOverlap`
  (params (OverlappedComponent :type "PrimitiveComponent Object Reference") (OtherActor :type "Actor Object Reference") (OtherComp :type "PrimitiveComponent Object Reference") (OtherBodyIndex :type Integer) (bFromSweep :type Boolean) (SweepResult :type "HitResult Structure (by ref)"))
  (bind _playerloc (`self.PlayerLoc`))
  (bind _playerrot (`self.PlayerRot`))
  ;[1 1 1] Check if level is cleared
  (if (`self.Load`)
    (`|ExecutionSequence`
      (:`then_0`
        ;[1 1 1] Set checkpoint is reached
        (bind _asthird_person_character (cast `/Game/ThirdPersonBP/Blueprints/ThirdPersonCharacter` (`GameplayStatics.GetPlayerCharacter` 0)))
        (`|ExecutionSequence`
          (:`then_0`
            (set `self.PlayerLoc` (`self.K2_GetActorLocation` _asthird_person_character))
            (`KismetSystemLibrary.PrintString` "Checkpoint Saved"))
          (:`then_1`
            (set `self.PlayerRot` (`self.K2_GetActorRotation` _asthird_person_character)))))
      (:`then_1`
        (bind _returnvalue (`GameplayStatics.DoesSaveGameExist` "check"))
        (if _returnvalue
          ;[1 1 1] Saves if there is already a save file
          (bind _returnvalue_2 (`GameplayStatics.LoadGameFromSlot` "check"))
          (bind _assave (cast `/Game/Checkpoints/Save` _returnvalue_2))
          (set `/Game/Checkpoints/Save.PlayerLocation` _playerloc _assave)
          (set `/Game/Checkpoints/Save.Player Rotation` _playerrot _assave)
          (set `/Game/Checkpoints/Save.load` true _assave)
          (`GameplayStatics.SaveGameToSlot` _assave "check")
          (else
            ;[1 1 1] Create a save file and saves
            (bind _returnvalue_3 (`GameplayStatics.CreateSaveGameObject` "/Game/Checkpoints/Save.Save_C"))
            (set `/Game/Checkpoints/Save.PlayerLocation` _playerloc _returnvalue_3)
            (set `/Game/Checkpoints/Save.Player Rotation` _playerrot _returnvalue_3)
            (set `/Game/Checkpoints/Save.load` true _returnvalue_3)
            (`GameplayStatics.SaveGameToSlot` _returnvalue_3 "check")))
        (`KismetSystemLibrary.Delay` 0.2)
        ;[1 1 1] Destroys checkpoint if checkpoint was already reached at one point.
        (`self.K2_DestroyActor`)))
    (else
      (bind _returnvalue_4 (`GameplayStatics.LoadGameFromSlot` "check"))
      ;[1 1 1] Reset the cleared level
      (bind _assave_2 (cast `/Game/Checkpoints/Save` _returnvalue_4))
      (set `/Game/Checkpoints/Save.load` false _assave_2)
      (`GameplayStatics.SaveGameToSlot` _assave_2 "check")
      (`KismetSystemLibrary.PrintString` "Checkpoint Cleared"))))

(fn `UserConstructionScript`)