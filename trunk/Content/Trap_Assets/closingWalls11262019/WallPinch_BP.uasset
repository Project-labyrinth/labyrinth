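; Pinching wall trap: when the Player class enters its box trigger, this wall and a referenced OppositeWall close toward each other.
; The overlap stores both world locations and moves both walls over TimeToClose to their Y midpoint, using the first wall's X and Z.
; After the second move and a delay, a return event moves both back to the stored positions.
; Stored world locations are passed directly as MoveComponentTo relative targets.
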(event `self.Box.OnComponentHit`
  (params (HitComponent :type "PrimitiveComponent Object Reference") (OtherActor :type "Actor Object Reference") (OtherComp :type "PrimitiveComponent Object Reference") (NormalImpulse :type "Vector Structure") (Hit :type "HitResult Structure (by ref)")))

(event `self.Box.OnComponentBeginOverlap`
  (params (OverlappedComponent :type "PrimitiveComponent Object Reference") (OtherActor :type "Actor Object Reference") (OtherComp :type "PrimitiveComponent Object Reference") (OtherBodyIndex :type Integer) (bFromSweep :type Boolean) (SweepResult :type "HitResult Structure (by ref)"))
  (bind _staticmeshcomponent (`self.StaticMeshComponent`))
  (bind (_wall2vector_x _wall2vector_y) (`KismetMathLibrary.BreakVector` (`self.wall2vector`)))
  (bind (_wall1vector_x _wall1vector_y _wall1vector_z) (`KismetMathLibrary.BreakVector` (`self.wall1vector`)))
  (bind (_wall1vector_x_2 _wall1vector_y_2) (`KismetMathLibrary.BreakVector` (`self.wall1vector`)))
  (bind (_wall2vector_x_2 _wall2vector_y_2) (`KismetMathLibrary.BreakVector` (`self.wall2vector`)))
  (bind (_wall1vector_x_3 _wall1vector_y_3 _wall1vector_z_2) (`KismetMathLibrary.BreakVector` (`self.wall1vector`)))
  (bind (_wall1vector_x_4 _wall1vector_y_4) (`KismetMathLibrary.BreakVector` (`self.wall1vector`)))
  (bind _rootcomponent (`Actor.RootComponent` (`self.Opposite Wall`)))
  (if (== (`GameplayStatics.GetObjectClass` OtherActor) (`self.Player`))
    (set `self.wall1vector` (`SceneComponent.K2_GetComponentLocation` _staticmeshcomponent))
    (set `self.wall2vector` (`SceneComponent.K2_GetComponentLocation` _rootcomponent))
    (`|ExecutionSequence`
      (:`then_0`
        (`KismetSystemLibrary.MoveComponentTo` _staticmeshcomponent (`KismetMathLibrary.MakeVector` _wall1vector_x (+ (/ (- _wall2vector_y _wall1vector_y_4) 2.0) _wall1vector_y) _wall1vector_z) (struct) false false (`self.TimeToClose`)))
      (:`then_1`
        (`KismetSystemLibrary.MoveComponentTo` _rootcomponent (`KismetMathLibrary.MakeVector` _wall1vector_x_3 (+ (/ (- _wall2vector_y_2 _wall1vector_y_2) 2.0) _wall1vector_y_3) _wall1vector_z_2) (struct) false false (`self.TimeToClose`))
        (`KismetSystemLibrary.Delay` (`self.delay`))
        (`self.return`)))))

(event `return`
  (`|ExecutionSequence`
    (:`then_0`
      (`KismetSystemLibrary.MoveComponentTo` (`self.StaticMeshComponent`) (`self.wall1vector`) (struct) false false (`self.TimeToClose`)))
    (:`then_1`
      (`KismetSystemLibrary.MoveComponentTo` (`Actor.RootComponent` (`self.Opposite Wall`)) (`self.wall2vector`) (struct) false false (`self.TimeToClose`)))))

(fn `UserConstructionScript`)